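; BP_Planet is a planet actor that orbits whatever component it is attached to, with configurable size, look and orbit speed.
; Each Tick rotates its offset from the first parent component around the yaw axis by Rotation scaled by delta time, then moves the actor there without sweeping.
; The construction script applies the uniform Scale and the Material.
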(event EventBeginPlay)

(event EventActorBeginOverlap
  (params (OtherActor :type Actor%20Object%20Reference)))

(event EventTick
  (params (DeltaSeconds :type Float%20%28single-precision%29))
  (Variables|Default|SetDeltaTime DeltaSeconds)
  (for (_array_element _array_index) (Class|SceneComponent|GetParentComponents)
    (if (== _array_index 0)
      (Utilities|IsValid _array_element
        (:Is%20Valid
          (Transformation|SetActorLocation (+ (Transformation|GetWorldLocation _array_element) (Math|Vector|RotateVector (- (Transformation|GetActorLocation) (Transformation|GetWorldLocation _array_element)) (Math|Rotator|MakeRotator 0.0 (* (Variables|Default|GetDeltaTime) (Variables|Default|GetRotation)) 0.0))) false))))))

(fn ConstructionScript
  (bind _scale (Variables|Default|GetScale))
  (Transformation|SetActorScale3D (Math|Vector|MakeVector _scale _scale _scale))
  (Rendering|Material|SetMaterial 0 (Variables|Default|GetMaterial)))