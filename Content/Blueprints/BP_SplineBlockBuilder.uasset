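; BP_SplineBlockBuilder is a construction-time tool actor that lines a spline with repeated copies of a static mesh.
; The construction script divides the spline length by LengthInterval and adds a Static Mesh component at each step, attached to the spline.
; Each component takes the spline's world location and rotation at that distance, plus a shared Material and uniform Scale.
; The event graph is empty, so nothing runs during play.
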(event EventBeginPlay)

(event EventActorBeginOverlap
  (params (OtherActor :type Actor%20Object%20Reference)))

(event EventTick
  (params (DeltaSeconds :type Float%20%28single-precision%29)))

(fn ConstructionScript
  (bind _scale (Variables|Default|GetScale))
  (for _index (range 0 (Math|Float|Floor (/ (Spline|GetSplineLength) (Variables|Default|GetLengthInterval))))
    (bind _returnvalue (AddComponent|AddStaticMeshComponent false))
    (Components|StaticMesh|SetStaticMesh _returnvalue (Variables|Default|GetMesh))
    (Class|SceneComponent|Attachto (Variables|Default|GetSpline) "None" "KeepRelativeOffset" true)
    (Transformation|SetWorldLocation _returnvalue (Class|SplineComponent|GetWorldLocationatDistanceAlongSpline (* _index (Variables|Default|GetLengthInterval))) false)
    (Transformation|SetWorldRotation _returnvalue (Class|SplineComponent|GetWorldRotationatDistanceAlongSpline (* _index (Variables|Default|GetLengthInterval))) false)
    (Rendering|Material|SetMaterial _returnvalue 0 (Variables|Default|GetMaterial))
    (Transformation|SetWorldScale3D _returnvalue (Math|Vector|MakeVector _scale _scale _scale))))