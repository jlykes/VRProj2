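; BP_Tile_Generator is a Blueprint that builds a grid of static mesh tiles in its construction script.
; Nested loops over Y and X add a mesh component per cell, attached to Origin, spaced by Space and uniformly sized by Scale.
; Each tile gets a random height offset and random pitch, yaw and roll, centred on zero within the HeightVariation and RotationVariation ranges.
; The event graph has no active logic.
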(event EventBeginPlay)

(event EventActorBeginOverlap
  (params (OtherActor :type Actor%20Object%20Reference)))

(event EventTick
  (params (DeltaSeconds :type Float%20%28single-precision%29)))

(fn ConstructionScript
  (bind _rotation_variation (Variables|Default|GetRotation%20Variation))
  (bind _scale (Variables|Default|GetScale))
  (bind _height_variation (Variables|Default|GetHeight%20Variation))
  (bind _returnvalue (/ _height_variation 2.0))
  (bind _returnvalue_2 (/ _rotation_variation 2.0))
  (bind _returnvalue_3 (* -1 _returnvalue_2))
  (for _index (range 0 (Variables|Default|GetY))
    (for _index_2 (range 0 (Variables|Default|GetX))
      (bind _returnvalue_4 (AddComponent|AddStaticMeshComponent false))
      (Class|SceneComponent|Attachto _returnvalue_4 (Variables|Default|GetOrigin) "None" "KeepRelativeOffset" true)
      (Transformation|SetRelativeLocation _returnvalue_4 (Math|Vector|MakeVector (* _index_2 (Variables|Default|GetSpace)) (* _index (Variables|Default|GetSpace)) (Math|Random|RandomFloatinRange (* -1 _returnvalue) _returnvalue)) false)
      (Transformation|SetWorldScale3D _returnvalue_4 (Math|Vector|MakeVector _scale _scale _scale))
      (Transformation|SetRelativeRotation _returnvalue_4 (Math|Rotator|MakeRotator (Math|Random|RandomFloatinRange _returnvalue_3 _returnvalue_2) (Math|Random|RandomFloatinRange _returnvalue_3 _returnvalue_2) (Math|Random|RandomFloatinRange _returnvalue_3 _returnvalue_2)) false))))